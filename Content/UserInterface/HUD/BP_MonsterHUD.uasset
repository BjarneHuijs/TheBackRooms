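; BP_MonsterHUD sets up the on-screen HUD, presumably for the monster player, with blood meter, ability and score system widgets.
; On BeginPlay it calls Initialize, which creates each widget for player controller 0 and adds it to the viewport.
; Nodes that hide the mouse cursor and set game-only input are present but disconnected, so they never run.
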(event `self.ReceiveBeginPlay`
  (`self.Initialize`))

(event `Initialize`
  (bind _returnvalue (`GameplayStatics.GetPlayerController` 0))
  (bind _returnvalue_2 (`|CreateWidget` "/Game/UserInterface/HUD/Widgets/BP_BloodMeterWidget.BP_BloodMeterWidget_C" _returnvalue))
  (`UserWidget.AddToViewport` _returnvalue_2 0)
  (bind _returnvalue_3 (`|CreateWidget` "/Game/UserInterface/HUD/Widgets/BP_AbilityWidget.BP_AbilityWidget_C" _returnvalue))
  (`UserWidget.AddToViewport` _returnvalue_3 0)
  (bind _returnvalue_4 (`|CreateWidget` "/Game/UserInterface/HUD/Widgets/BP_ScoreSystemWidget.BP_ScoreSystemWidget_C" _returnvalue))
  (`UserWidget.AddToViewport` _returnvalue_4 0))

(fn `UserConstructionScript`)