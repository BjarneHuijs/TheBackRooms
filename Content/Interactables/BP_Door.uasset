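; BP_Door is a door that rotates on a timer from BeginPlay, with no player interaction.
; BeginPlay sets DoorLocked, then clears it after a short delay.
; Tick polls that flag through DoOnce gates, playing the DoorMovement timeline while locked and reversing it from the end once unlocked.
; The timeline drives the Door's relative yaw; only the locked-side gate gets reset, so the reverse fires once.
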(event `self.ReceiveBeginPlay`
  (set `self.DoorLocked` true)
  (`KismetSystemLibrary.Delay` 5.0)
  (set `self.DoorLocked` false))

(event `self.ReceiveTick`
  (params (DeltaSeconds :type "Float (single-precision)"))
  (if (`self.DoorLocked`)
    (`/Engine/EditorBlueprintResources/StandardMacros.DoOnce` false :!label _label
      (:`Completed`
        (bind (_direction _dooropening) (`Timeline|DoorMovement` :!label _label_2)
          (:`Update`
            (`SceneComponent.K2_SetRelativeRotation` (`self.Door`) (`KismetMathLibrary.MakeRotator` 0.0 0.0 _dooropening) false false)))))
    (else
      (`|ExecutionSequence`
        (:`then_0`
          (goto _label :!via `Reset`))
        (:`then_1`
          (`/Engine/EditorBlueprintResources/StandardMacros.DoOnce` false
            (:`Completed`
              (goto _label_2 :!via `ReverseFromEnd`))))))))

(fn `UserConstructionScript`)