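; Lockable double door that swings its two door meshes open or closed according to the MIsClosed flag, which this graph only reads.
; Tick polls the flag, using DoOnce gates to trigger two timelines that drive each mesh's relative yaw.
; Closing reverses both timelines from the end and opening plays them forward.
; The open state re-arms the close gate, while timeline completion re-arms the open gates.
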(event `self.ReceiveTick`
  (params (DeltaSeconds :type "Float (single-precision)"))
  (if (`self.m_IsClosed`)
    (`/Engine/EditorBlueprintResources/StandardMacros.DoOnce` false :!label _label
      (:`Completed`
        (`|ExecutionSequence`
          (:`then_0`
            (bind (_direction _doorrotation) (`Timeline|DoorMovement2` :!via `ReverseFromEnd` :!label _label_2)
              (:`Update`
                (`SceneComponent.K2_SetRelativeRotation` (`self.LockDoor1`) (`KismetMathLibrary.MakeRotator` 0.0 0.0 _doorrotation) false false))
              (:`Finished`
                (goto _label_5 :!via `Reset`))))
          (:`then_1`
            (bind (_direction_2 _dooropening) (`Timeline|DoorMovement` :!via `ReverseFromEnd` :!label _label_3)
              (:`Update`
                (`SceneComponent.K2_SetRelativeRotation` (`self.LockDoor`) (`KismetMathLibrary.MakeRotator` 0.0 0.0 _dooropening) false false))
              (:`Finished`
                (goto _label_4 :!via `Reset`)))))))
    (else
      (`|ExecutionSequence`
        (:`then_0`
          (goto _label :!via `Reset`))
        (:`then_1`
          (`/Engine/EditorBlueprintResources/StandardMacros.DoOnce` true :!label _label_4
            (:`Completed`
              (goto _label_3))))
        (:`then_2`
          (`/Engine/EditorBlueprintResources/StandardMacros.DoOnce` true :!label _label_5
            (:`Completed`
              (goto _label_2))))))))

(fn `UserConstructionScript`)