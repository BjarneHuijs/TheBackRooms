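; Game mode for the Backrooms menu levels that handles the player pawn and the high score prompt.
; On BeginPlay it hides, disables and stops ticking the controlled pawn, and shows its root component tree only in ShowCaseLevel.
; Tick watches a MyPlayerMonster pawn and opens the high score adder once when it dies.
; The construction script assigns the pause and new record menu widget classes.
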(event `self.ReceiveBeginPlay`
  (bind _returnvalue (`GameplayStatics.GetPlayerController` 0))
  (bind _returnvalue_2 (`Controller.K2_GetPawn` _returnvalue))
  (`self.SetActorHiddenInGame` _returnvalue_2 true)
  (`self.SetActorTickEnabled` _returnvalue_2 false)
  (`self.DisableInput` _returnvalue_2 _returnvalue)
  (bind _returnvalue_3 (`GameplayStatics.GetCurrentLevelName` true))
  (if (`KismetStringLibrary.EqualEqual_StrStr` _returnvalue_3 "ShowCaseLevel")
    (`SceneComponent.SetHiddenInGame` (`self.DefaultSceneRoot`) false true)
    (else
      (`SceneComponent.SetHiddenInGame` (`self.DefaultSceneRoot`) true true))))

(event `self.ReceiveTick`
  (params (DeltaSeconds :type "Float (single-precision)"))
  (bind _asmy_player_monster (cast `/Game/Monster/MyPlayerMonster` (`Controller.K2_GetPawn` (`GameplayStatics.GetPlayerController` 0))))
  (if (`PlayerMonster.IsDead` _asmy_player_monster)
    (`/Engine/EditorBlueprintResources/StandardMacros.DoOnce` false
      (:`Completed`
        (`self.OpenHighScoreAdder`)))))

(fn `UserConstructionScript`
  (set `self.m_PauseClass` "/Game/UserInterface/Menus/Widgets/BP_PauseMenu.BP_PauseMenu_C")
  (set `self.m_NewScoreClass` "/Game/UserInterface/Menus/Widgets/BP_NewRecordMenu.BP_NewRecordMenu_C"))