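; Game mode for the Backrooms game that opens the high score entry when the player's monster pawn dies.
; Tick polls the controlled MyPlayerMonster for death and calls OpenHighScoreAdder once through a DoOnce.
; The construction script assigns the pause menu and new record menu classes.
; BeginPlay unhides the root component hierarchy only in ShowCaseLevel, and an unconnected game-only input snippet never runs.
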(event `self.ReceiveBeginPlay`
  (bind _returnvalue (`GameplayStatics.GetCurrentLevelName` true))
  (if (`KismetStringLibrary.EqualEqual_StrStr` _returnvalue "ShowCaseLevel")
    (`SceneComponent.SetHiddenInGame` (`self.DefaultSceneRoot`) false true)
    (else
      (`SceneComponent.SetHiddenInGame` (`self.DefaultSceneRoot`) true true))))

(event `self.ReceiveTick`
  (params (DeltaSeconds :type "Float (single-precision)"))
  (bind _asmy_player_monster (cast `/Game/Monster/MyPlayerMonster` (`Controller.K2_GetPawn` (`GameplayStatics.GetPlayerController` 0))))
  (if (`PlayerMonster.IsDead` _asmy_player_monster)
    (`/Engine/EditorBlueprintResources/StandardMacros.DoOnce` false
      (:`Completed`
        (`self.OpenHighScoreAdder`)))))

(fn `UserConstructionScript`
  (set `self.m_PauseClass` "/Game/UserInterface/Menus/Widgets/BP_PauseMenu.BP_PauseMenu_C")
  (set `self.m_NewScoreClass` "/Game/UserInterface/Menus/Widgets/BP_NewRecordMenu.BP_NewRecordMenu_C"))